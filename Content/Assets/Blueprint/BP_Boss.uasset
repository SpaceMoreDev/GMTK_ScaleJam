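; Boss character with two child-actor arms posed from its skeletal mesh, a W_Boss UI widget and Behavior Tree-facing state.
; Tick turns low arm values into hit and stun flags, copying them to the blackboard only while alive and below a health threshold.
; Damage lowers health and counts hits to unlock a smash.
; PlayerAttacked hurts a grounded player, or, through a DoOnce, launches an airborne one and damages the boss.
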(event `self.ReceiveBeginPlay`
  (`|ExecutionSequence`
    (:`then_0`
      (bind _astop_down_character (cast `/Game/Assets/Blueprint/TopDownCharacter` (`GameplayStatics.GetPlayerCharacter` 0)))
      (set `self.Player` _astop_down_character))
    (:`then_1`
      (bind _returnvalue (`|CreateWidget` "/Game/Assets/Blueprint/W_Boss.W_Boss_C" (`GameplayStatics.GetPlayerController` 0)))
      (set `/Game/Assets/Blueprint/W_Boss.Boss` self _returnvalue)
      (`UserWidget.AddToViewport` _returnvalue 0))))

(event `self.ReceiveTick`
  (params (DeltaSeconds :type "Float (single-precision)"))
  (bind _returnvalue (`AIBlueprintHelperLibrary.GetBlackboard` (`AIBlueprintHelperLibrary.GetAIController` self)))
  (if (not (`self.isDead`))
    (`|ExecutionSequence`
      (:`then_0`
        (if (< (`self.ArmR`) 0.5)
          (set `self.ableToHit_L` true)
          (set `self.ableToHit_R` false)
          (set `self.isStunned_R` true)
          (elif (< (`self.ArmL`) 0.5)
            (set `self.ableToHit_L` false)
            (set `self.ableToHit_R` true)
            (set `self.isStunned_L` true))))
      (:`then_1`
        (if (< (`self.Health`) 50.0)
          (`BlackboardComponent.SetValueAsBool` _returnvalue "canHit_L" (`self.ableToHit_L`))
          (`BlackboardComponent.SetValueAsBool` _returnvalue "canHit_R" (`self.ableToHit_R`))
          (`BlackboardComponent.SetValueAsBool` _returnvalue "stunned_L" (`self.isStunned_L`))
          (`BlackboardComponent.SetValueAsBool` _returnvalue "stunned_R" (`self.isStunned_R`))
          (`BlackboardComponent.SetValueAsBool` _returnvalue "canSmash" (`self.canSmashnow`))
          (`BlackboardComponent.SetValueAsBool` _returnvalue "dead" (`self.isDead`)))))))

(event `self.ReceiveAnyDamage`
  (params (Damage :type "Float (single-precision)") (DamageType :type "DamageType Object Reference") (InstigatedBy :type "Controller Object Reference") (DamageCauser :type "Actor Object Reference"))
  (bind _output_get (set `self.Health` (- (`self.Health`) Damage)))
  (if (<= _output_get 0.0)
    (set `self.isDead` true)
    (set `self.canSmashnow` false)
    (else
      (bind _result (`/Engine/EditorBlueprintResources/StandardMacros.IncrementFloat` (`self.damagecounter`))
        (:`  `
          (bind _output_get_2 (set `self.damagecounter` _result))
          (`KismetSystemLibrary.PrintString` (`KismetStringLibrary.Conv_DoubleToString` _output_get_2))
          (if (>= _output_get_2 (`self.smash_damage_threshold`))
            (set `self.canSmashnow` true)))))))

(fn `PlayerAttacked`
  (params (Actor :type "Character Object Reference"))
  (if (`NavMovementComponent.IsMovingOnGround` (`Character.CharacterMovement` (`self.player`)))
    (`GameplayStatics.ApplyDamage` (`self.player`) 1.0 null self)
    (else
      (`/Engine/EditorBlueprintResources/StandardMacros.DoOnce` false
        (:`Completed`
          (`Character.LaunchCharacter` (`self.player`) (0.0 0.0 500.0) false true)
          (`GameplayStatics.ApplyDamage` self 10.0 null (`self.player`)))))))

(fn `UserConstructionScript`
  (`SkinnedMeshComponent.SetLeaderPoseComponent` (`self.GetComponentByClass` (`ChildActorComponent.ChildActor` (`self.Arm`)) "/Script/Engine.SkeletalMeshComponent") (`self.SkeletalMesh`) false)
  (`SkinnedMeshComponent.SetLeaderPoseComponent` (`self.GetComponentByClass` (`ChildActorComponent.ChildActor` (`self.Arm1`)) "/Script/Engine.SkeletalMeshComponent") (`self.SkeletalMesh`) false))