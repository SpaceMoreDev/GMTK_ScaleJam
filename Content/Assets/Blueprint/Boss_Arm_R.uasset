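; Right arm of the boss, a child actor of BP_Boss that attacks the player and can be scaled.
; Two hit boxes store an overlapping TopDownCharacter and call PlayerAttacked.
; The ScaleSkeletal override mirrors in-range scale values to the boss's ArmR.
; While the living boss has this arm stunned, Tick grows ArmR and CurrentScale back toward full size, then clears the stun.
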(event `self.ReceiveBeginPlay`
  (`parent.ReceiveBeginPlay`)
  (set `self.scaleSkeleton` true)
  (bind _asbp_boss (cast `/Game/Assets/Blueprint/BP_Boss` (`self.GetParentActor`)))
  (set `self.Boss` _asbp_boss))

(event `self.ReceiveTick`
  (params (DeltaSeconds :type "Float (single-precision)"))
  (bind _boss (`self.Boss`))
  (bind _returnvalue (+ (`/Game/Assets/Blueprint/BP_Boss.ArmR` _boss) (* (`GameplayStatics.GetWorldDeltaSeconds`) (`self.Restore Speed`))))
  (`parent.ReceiveTick` DeltaSeconds)
  (if (`/Game/Assets/Blueprint/BP_Boss.isDead` (`self.Boss`))
    _
    (elif (`/Game/Assets/Blueprint/BP_Boss.isStunned_R` (`self.Boss`))
      (if (< _returnvalue 1.0)
        (bind _output_get (set `/Game/Assets/Blueprint/BP_Boss.ArmR` _returnvalue _boss))
        (set `self.current_scale` (`KismetMathLibrary.Conv_DoubleToVector` _output_get))
        (else
          (set `/Game/Assets/Blueprint/BP_Boss.isStunned_R` false _boss))))))

(event `self.Box3.OnComponentBeginOverlap`
  (params (OverlappedComponent :type "PrimitiveComponent Object Reference") (OtherActor :type "Actor Object Reference") (OtherComp :type "PrimitiveComponent Object Reference") (OtherBodyIndex :type Integer) (bFromSweep :type Boolean) (SweepResult :type "HitResult Structure (by ref)"))
  (bind _astop_down_character (cast `/Game/Assets/Blueprint/TopDownCharacter` OtherActor))
  (set `self.player` _astop_down_character)
  (`self.PlayerAttacked` null :!label _label))

(event `self.Box1.OnComponentBeginOverlap`
  (params (OverlappedComponent :type "PrimitiveComponent Object Reference") (OtherActor :type "Actor Object Reference") (OtherComp :type "PrimitiveComponent Object Reference") (OtherBodyIndex :type Integer) (bFromSweep :type Boolean) (SweepResult :type "HitResult Structure (by ref)"))
  (bind _astop_down_character (cast `/Game/Assets/Blueprint/TopDownCharacter` OtherActor))
  (set `self.player` _astop_down_character)
  (goto _label))

(fn `ScaleSkeletal`
  (params (`new scale` :type "Vector Structure"))
  (bind _x (.x `new scale`))
  (`parent.ScaleSkeletal` `new scale`)
  (if (and (< _x (`self.Up_Scale`)) (> _x (`self.Down_Scale`)))
    (set `/Game/Assets/Blueprint/BP_Boss.ArmR` _x (`self.Boss`))))

(fn `UserConstructionScript`
  (`parent.UserConstructionScript`))