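; Boss arm actor that resolves player attacks on behalf of its parent actor, presumably the boss.
; PlayerAttacked damages the player if they are moving on the ground; otherwise, a DoOnce with no visible reset launches them upward and damages the parent actor.
; BeginPlay runs the parent logic and enables the ScaleSkeleton flag, while the ScaleSkeletal function is empty.
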(event `self.ReceiveBeginPlay`
  (`parent.ReceiveBeginPlay`)
  (set `self.scaleSkeleton` true))

(fn `PlayerAttacked`
  (params (Actor :type "Character Object Reference"))
  (if (`NavMovementComponent.IsMovingOnGround` (`Character.CharacterMovement` (`self.player`)))
    (`GameplayStatics.ApplyDamage` (`self.player`) 1.0 null (`self.GetParentActor`))
    (else
      (`/Engine/EditorBlueprintResources/StandardMacros.DoOnce` false
        (:`Completed`
          (`Character.LaunchCharacter` (`self.player`) (0.0 0.0 1000.0) false true)
          (`GameplayStatics.ApplyDamage` (`self.GetParentActor`) 10.0 null (`self.player`)))))))

(fn `ScaleSkeletal`
  (params (`new scale` :type "Vector Structure")))

(fn `UserConstructionScript`
  (`parent.UserConstructionScript`))