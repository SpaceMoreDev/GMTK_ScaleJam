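; ScaleObject is an actor Blueprint that temporarily shrinks or enlarges itself when StartScaling is triggered.
; The Shrink flag selects DownScale or UpScale, which the Scale function multiplies into the current actor scale, returning the previous scale.
; After ScaleDelay, the event restores that saved scale.
; IsScaled is true during the effect but is not checked here to block repeat triggers.
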(event `StartScaling`
  (params (Shrink :type Boolean))
  (bind _scale_delay (`self.Scale_Delay`))
  (set `self.IsScaled` true)
  (if Shrink
    (bind _original_scale (`self.Scale` (`self.Down_Scale`)))
    (`KismetSystemLibrary.Delay` _scale_delay)
    (`self.SetActorScale3D` _original_scale)
    (else
      (bind _original_scale_2 (`self.Scale` (`self.Up_Scale`)))
      (`KismetSystemLibrary.Delay` _scale_delay)
      (`self.SetActorScale3D` _original_scale_2)))
  (set `self.IsScaled` false))

(fn `Scale`
  (params (Scale :type "Float (double-precision)"))
  (returns (`Original Scale` :type "Vector Structure"))
  (locals (Temp :type "Vector Structure"))
  (bind _output_get (set `local.Temp` (`self.GetActorScale3D`)))
  (`self.SetActorScale3D` (* _output_get Scale))
  (return _output_get))

(fn `UserConstructionScript`)