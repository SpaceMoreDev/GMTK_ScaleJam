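; BP_Enemy is an enemy that chases the player and can be killed by jumping on it.
; Each Tick it moves horizontally toward a nearby player who is not well above it, using an unswept, frame-rate-dependent offset.
; On collision overlap, a grounded TopDownCharacter loses health and respawns through TopDownGameMode, while an airborne one is launched upward and destroys the enemy.
; A level-reload branch is left unconnected.
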(event `self.ReceiveBeginPlay`)

(event `self.ReceiveTick`
  (params (DeltaSeconds :type "Float (single-precision)"))
  (bind _returnvalue (`self.K2_GetActorLocation`))
  (bind _returnvalue_2 (`self.K2_GetActorLocation` (`GameplayStatics.GetPlayerPawn` 0)))
  (if (and (< (`KismetMathLibrary.Vector_Distance` _returnvalue_2 _returnvalue) 700.0) (< (.z _returnvalue_2) (+ (.z _returnvalue) 50.0)))
    (`self.K2_AddActorWorldOffset` (* (* (`KismetMathLibrary.Normal` (- (`self.K2_GetActorLocation` (`GameplayStatics.GetPlayerPawn` 0)) (`self.K2_GetActorLocation`))) (1.0 1.0 0.0)) (`self.Speed`)))))

(event `self.Collision.OnComponentBeginOverlap`
  (params (OverlappedComponent :type "PrimitiveComponent Object Reference") (OtherActor :type "Actor Object Reference") (OtherComp :type "PrimitiveComponent Object Reference") (OtherBodyIndex :type Integer) (bFromSweep :type Boolean) (SweepResult :type "HitResult Structure (by ref)"))
  (bind _astop_down_character (cast `/Game/Assets/Blueprint/TopDownCharacter` OtherActor))
  (if (`NavMovementComponent.IsMovingOnGround` (`Character.CharacterMovement` _astop_down_character))
    (bind _astop_down_game_mode (cast `/Game/Assets/Blueprint/TopDownGameMode` (`GameplayStatics.GetGameMode`)))
    (`/Game/Assets/Blueprint/TopDownCharacter.decrease Health` _astop_down_character)
    (`/Game/Assets/Blueprint/TopDownGameMode.Respawn Player` _astop_down_game_mode)
    (else
      (`KismetSystemLibrary.PrintString` "Hello")
      (`Character.LaunchCharacter` _astop_down_character (`KismetMathLibrary.MakeVector` 0.0 0.0 (`self.JumpBounce`)) false false)
      (`self.K2_DestroyActor`))))

(fn `UserConstructionScript`)